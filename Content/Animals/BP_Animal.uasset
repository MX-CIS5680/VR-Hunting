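; Base animal character that manages health, energy and rest for an AI-controlled creature.
; Tick drains energy, or regains it while resting, and sets the blackboard rest flag when nearly empty.
; Damage reduces health; death stops movement and brain logic.
; Timed rest and hunter-reaction events end through a delayed finish dispatch, while MoveToLocation and DecideDestination are placeholders.
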(event `self.ReceiveBeginPlay`
  (set `self.energy` (`self.MAX_ENERGY`))
  (set `self.health` (`self.MAX_HEALTH`))
  (bind _output_get (set `self.blackBoard` (`AIBlueprintHelperLibrary.GetBlackboard` null)))
  (`/Engine/EditorBlueprintResources/StandardMacros.IsValid` _output_get
    (:`Is Valid`
      _)
    (:`Is Not Valid`
      _))
  (`KismetSystemLibrary.PrintString` "InvalidBlackBoardInBP_ANIMAL"))

(event `self.ReceiveTick`
  (params (DeltaSeconds :type "Float (single-precision)"))
  (`self.UpdateEnergy` DeltaSeconds)
  (if (not (`self.needRest`))
    (if (< (`self.energy`) 1.0)
      (`self.SetNeedRest` true))))

(event `Die`
  (`MovementComponent.StopMovementImmediately` (`self.CharacterMovement`))
  (bind _asaicontroller (cast `AIController` (`self.GetController`)))
  (`BrainComponent.StopLogic` (`AIController.BrainComponent` _asaicontroller) ""))

(event `TakeDamage`
  (params (DMG :type "Float (double-precision)") (Source :type "Actor Object Reference"))
  (`self.SetHealth` (- (`self.health`) DMG))
  (if (<= (`self.health`) 0.0)
    (`self.Die`)))

(event `GoToRest`
  (`MovementComponent.StopMovementImmediately` (`self.CharacterMovement`))
  (set `self.state` "NewEnumerator1")
  (`KismetSystemLibrary.Delay` (`self.restTime`))
  (set `self.state` "NewEnumerator0")
  (`self.SetNeedRest` false)
  (`self.EndAction`))

(event `ReactToHunter`
  (params (Hunter :type "Actor Object Reference"))
  (`KismetSystemLibrary.Delay` 5.0)
  (`KismetSystemLibrary.PrintString` "Finish Reaction in BP")
  (`self.EndAction`))

(event `MoveToLocation`
  (params (Location :type "Vector Structure")))

(event `EndAction`
  (`KismetSystemLibrary.Delay` (`self.reactionTime`))
  (`KismetSystemLibrary.PrintString` "SendFinishActionDispatch")
  (`self.FinishTimeCostingEvent`))

(fn `DecideDestination`
  (returns (location :type "Vector Structure"))
  (return (0.0 0.0 0.0)))

(fn `SetEnergy`
  (params (newVal :type "Float (double-precision)"))
  (set `self.energy` (`KismetMathLibrary.FClamp` newVal 0.0 (`self.MAX_ENERGY`))))

(fn `SetHealth`
  (params (newVal :type "Float (double-precision)"))
  (set `self.health` (`KismetMathLibrary.FClamp` newVal 0.0 (`self.MAX_HEALTH`))))

(fn `SetNeedRest`
  (params (`NeedRest?` :type Boolean))
  (locals (NewLocalVar :type Name :default "NeedRest"))
  (`BlackboardComponent.SetValueAsBool` (`self.blackBoard`) (`local.NewLocalVar`) `NeedRest?`)
  (set `self.needRest` `NeedRest?`))

(fn `SetNeedRun`
  (params (`needRun?` :type Boolean))
  (locals (NewLocalVar_0 :type Name :default "NeedRun"))
  (`BlackboardComponent.SetValueAsBool` (`self.blackBoard`) (`local.NewLocalVar_0`) `needRun?`)
  (set `self.needRun` `needRun?`))

(fn `UpdateEnergy`
  (params (deltaTime :type "Float (double-precision)"))
  (if (`|EnumEquality` (`self.state`) "NewEnumerator1")
    (`self.SetEnergy` (+ (* deltaTime (`self.regainEnergy`)) (`self.energy`)))
    (else
      (`self.SetEnergy` (- (`self.energy`) (* (`self.costEnergy`) deltaTime))))))

(fn `UserConstructionScript`)
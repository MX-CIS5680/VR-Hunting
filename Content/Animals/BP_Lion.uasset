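; BP_Lion is an AI animal, extending a parent class, that wanders, rests and charges the hunter, stored on the Blackboard as the player pawn.
; On reacting, it stops, roars, runs to the hunter, then plays a bite even if the move fails, applying no damage here.
; Damage halts it and low health sets NeedRun, which raises move speed and widens the random navmesh destination radius.
; One-shot animations temporarily override ABP_Lion, which StopAnimation restores.
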(event `self.ReceiveBeginPlay`
  (`parent.ReceiveBeginPlay`)
  (`BlackboardComponent.SetValueAsObject` (`self.blackBoard`) (`self.HunterKey`) (`GameplayStatics.GetPlayerPawn` 0)))

(event `self.TakeDamage`
  (params (DMG :type "Float (double-precision)") (Source :type "Actor Object Reference"))
  (`parent.TakeDamage` DMG Source)
  (set `self.state` "NewEnumerator0")
  (if (`self.needRun`)
    _
    (elif (< (`self.health`) 50.0)
      (`self.SetNeedRun` true)))
  (`MovementComponent.StopMovementImmediately` (`self.CharacterMovement`)))

(event `self.GoToRest`
  (set `self.restTime` (`KismetMathLibrary.RandomFloatInRange` 20.0 30.0))
  (`parent.GoToRest`))

(event `self.ReactToHunter`
  (params (Hunter :type "Actor Object Reference"))
  (`MovementComponent.StopMovementImmediately` (`self.CharacterMovement`))
  (set `self.state` "NewEnumerator0")
  (`SkeletalMeshComponent.PlayAnimation` (`self.Mesh`) "/Game/AfricanAnimalsPack/LionAndLioness/Animations/ANIM_Lion_Roar.ANIM_Lion_Roar" false)
  (`KismetSystemLibrary.Delay` 1.8)
  (`self.StopAnimation`)
  (set `CharacterMovementComponent.MaxWalkSpeed` (`self.RunSpeed`) (`self.CharacterMovement`))
  (`|AIMoveTo` self (0.0 0.0 0.0) Hunter
    (:`OnSuccess`
      _)
    (:`OnFail`
      _))
  (`SkeletalMeshComponent.PlayAnimation` (`self.Mesh`) "/Game/AfricanAnimalsPack/LionAndLioness/Animations/ANIM_Lion_Bite.ANIM_Lion_Bite" false)
  (set `CharacterMovementComponent.MaxWalkSpeed` (`self.WalkSpeed`) (`self.CharacterMovement`))
  (`KismetSystemLibrary.Delay` 1.0)
  (`self.StopAnimation`)
  (`self.EndAction`))

(event `self.MoveToLocation`
  (params (Location :type "Vector Structure"))
  (bind _charactermovement (`self.CharacterMovement`))
  (`|ExecutionSequence`
    (:`then_0`
      ;[1 1 1] Set Walk/Run Speed
      (if (`self.needRun`)
        (set `CharacterMovementComponent.MaxWalkSpeed` (`self.RunSpeed`) _charactermovement)
        (else
          (set `CharacterMovementComponent.MaxWalkSpeed` (`self.WalkSpeed`) _charactermovement))))
    (:`then_1`
      (`|AIMoveTo` self Location null
        (:`OnSuccess`
          (`self.SetNeedRun` false))
        (:`OnFail`
          (`KismetSystemLibrary.PrintString` "FailToMove")))
      (`self.EndAction`))))

(fn `DecideDestination`
  (returns (location :type "Vector Structure"))
  (locals (minRadius :type "Float (double-precision)") (maxRadius :type "Float (double-precision)") (selfLocation :type "Vector Structure"))
  (`|ExecutionSequence`
    (:`then_0`
      (set `local.selfLocation` (`self.K2_GetActorLocation`)))
    (:`then_1`
      (if (`self.needRun`)
        (set `local.minRadius` 800.0)
        (set `local.maxRadius` 1600.0)
        (else
          (set `local.minRadius` 400.0)
          (set `local.maxRadius` 700.0))))
    (:`then_2`
      (bind (_randomlocation _returnvalue) (`NavigationSystemV1.K2_GetRandomLocationInNavigableRadius` (`local.selfLocation`) (`KismetMathLibrary.RandomFloatInRange` (`local.minRadius`) (`local.maxRadius`)) null null))
      (if _returnvalue
        (return _randomlocation)))))

(fn `StopAnimation`
  (bind _mesh (`self.Mesh`))
  (`SkeletalMeshComponent.SetAnimationMode` _mesh "AnimationBlueprint" true)
  (`SkeletalMeshComponent.SetAnimInstanceClass` _mesh "/Game/Animals/Animation/ABP_Lion.ABP_Lion_C"))

(fn `UserConstructionScript`
  (`parent.UserConstructionScript`))
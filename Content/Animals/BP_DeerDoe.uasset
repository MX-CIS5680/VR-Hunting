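; BP_DeerDoe is a deer doe animal that roams at random using AIMoveTo to reachable nav points.
; Roaming starts on BeginPlay and repeats after a random pause on each successful arrival.
; AI Perception sets a panic flag on sensed stimuli, but RunAway, which sprints to a random point then resumes roaming, is not called here.
; Rest and BackToNormalMovement, also uncalled here, switch between a one-shot rest animation and the AnimBP.
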(event `self.ReceiveBeginPlay`
  (`TypedElementListLibrary.Reset` (struct))
  (`self.DecideNextAction` true))

(event `DecideNextAction`
  (params (SkipDelay :type Boolean))
  (if (not SkipDelay)
    (`KismetSystemLibrary.Delay` (`KismetMathLibrary.RandomFloatInRange` 1.0 5.0)))
  (`self.RandomRoam`))

(event `RandomRoam`
  ;[1 1 1] Random roam
  (set `CharacterMovementComponent.MaxWalkSpeed` (`self.WALK_SPEED`) (`self.CharacterMovement`))
  (`|AIMoveTo` self (`NavigationSystemV1.K2_GetRandomReachablePointInRadius` (`self.K2_GetActorLocation`) (`KismetMathLibrary.RandomFloatInRange` (`self.MIN_WANDER_RADIUS`) (`self.MAX_WANDER_RADIUS`)) null null) null
    (:`OnSuccess`
      (`self.DecideNextAction` false))))

(event `RunAway`
  ;[1 1 1] Run away
  (set `CharacterMovementComponent.MaxWalkSpeed` (`self.RUN_SPEED`) (`self.CharacterMovement`))
  (`|AIMoveTo` self (`NavigationSystemV1.K2_GetRandomReachablePointInRadius` (`self.K2_GetActorLocation`) (`KismetMathLibrary.RandomFloatInRange` (`self.MIN_RUN_RADIUS`) (`self.MAX_RUN_RADIUS`)) null null) null
    (:`OnSuccess`
      (set `self.InPanic` false)
      (`KismetSystemLibrary.PrintString` "StopRun")
      (`self.DecideNextAction` true))
    (:`OnFail`
      (`KismetSystemLibrary.PrintString` "FailToRun"))))

(event `Rest`
  (`MovementComponent.StopMovementImmediately` (`self.CharacterMovement`))
  (`SkeletalMeshComponent.PlayAnimation` (`self.Mesh`) "/Game/AnimalVarietyPack/DeerStagAndDoe/Animations/ANIM_DeerDoe_GoToRest.ANIM_DeerDoe_GoToRest" false)
  (`KismetSystemLibrary.Delay` 0.2))

(event `self.AIPerception.OnTargetPerceptionUpdated`
  (params (Actor :type "Actor Object Reference") (Stimulus :type "AIStimulus Structure"))
  ;[1 1 1] Detect Noise (use Report Noise Event in playerBP)
  (if (not (`self.InPanic`))
    (set `self.InPanic` (`.bSuccessfullySensed` (break `AIStimulus` Stimulus)))))

(fn `BackToNormalMovement`
  (bind _mesh (`self.Mesh`))
  (`SkeletalMeshComponent.SetAnimationMode` _mesh "AnimationBlueprint" true)
  (`SkeletalMeshComponent.SetAnimInstanceClass` _mesh "/Game/Animals/AnimBP_DeerDoe.AnimBP_DeerDoe_C"))

(fn `UserConstructionScript`)
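; Stag deer animal Blueprint that wanders the navmesh, rests, and flees when it reacts to a hunter or takes damage.
; Hunter reactions and damage change its state, set NeedRun and stop movement; moves set walk or run speed, use AIMoveTo, then end the action.
; DecideDestination picks a navigable point in a randomized forward arc, farther when running, falling back to a random point around itself.
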(event `self.ReceiveTick`
  (params (DeltaSeconds :type "Float (single-precision)"))
  (`parent.ReceiveTick` DeltaSeconds))

(event `self.MoveToLocation`
  (params (Location :type "Vector Structure"))
  (bind _charactermovement (`self.CharacterMovement`))
  (`|ExecutionSequence`
    (:`then_0`
      ;[1 1 1] Set Walk/Run Speed
      (if (`self.needRun`)
        (set `CharacterMovementComponent.MaxWalkSpeed` 600.0 _charactermovement)
        (else
          (set `CharacterMovementComponent.MaxWalkSpeed` 150.0 _charactermovement))))
    (:`then_1`
      (`|AIMoveTo` self Location null
        (:`OnSuccess`
          (`self.SetNeedRun` false))
        (:`OnFail`
          (`KismetSystemLibrary.PrintString` "FailToMove")))
      (`self.EndAction`))))

(event `self.GoToRest`
  (set `self.restTime` (`KismetMathLibrary.RandomFloatInRange` 5.0 10.0))
  (`parent.GoToRest`))

(event `self.ReactToHunter`
  (params (Hunter :type "Actor Object Reference"))
  (set `self.state` "NewEnumerator0")
  (`self.SetNeedRun` true)
  (`MovementComponent.StopMovementImmediately` (`self.CharacterMovement`)))

(event `self.TakeDamage`
  (params (DMG :type "Float (double-precision)") (Source :type "Actor Object Reference"))
  (`parent.TakeDamage` DMG Source)
  (set `self.state` "NewEnumerator0")
  (`self.SetNeedRun` true)
  (`MovementComponent.StopMovementImmediately` (`self.CharacterMovement`)))

(fn `DecideDestination`
  (returns (location :type "Vector Structure"))
  (locals (selfLocation :type "Vector Structure" :default (0.0 0.0 0.0)) (minRadius :type "Float (double-precision)" :default 0.0) (maxRadius :type "Float (double-precision)" :default 0.0) (NewLocalVar :type "Vector Structure"))
  (`|ExecutionSequence`
    (:`then_0`
      (set `local.selfLocation` (`self.K2_GetActorLocation`)))
    (:`then_1`
      (if (`self.needRun`)
        (set `local.minRadius` 2000.0)
        (set `local.maxRadius` 3000.0)
        (else
          (set `local.minRadius` 1000.0)
          (set `local.maxRadius` 1500.0))))
    (:`then_2`
      (bind (_randomlocation _returnvalue) (`NavigationSystemV1.K2_GetRandomLocationInNavigableRadius` (+ (`local.selfLocation`) (* (`KismetMathLibrary.Normal` (+ (`self.GetActorForwardVector`) (* (`self.GetActorRightVector`) (`KismetMathLibrary.RandomFloatInRange` -1.0 1.0)))) (`KismetMathLibrary.RandomFloatInRange` (`local.minRadius`) (`local.maxRadius`)))) (`KismetMathLibrary.RandomFloatInRange` 300.0 600.0) null null))
      (if _returnvalue
        (return _randomlocation)
        (else
          (bind _randomlocation_2 (`NavigationSystemV1.K2_GetRandomLocationInNavigableRadius` (`local.selfLocation`) (`KismetMathLibrary.RandomFloatInRange` (`local.minRadius`) (`local.maxRadius`)) null null))
          (return _randomlocation_2))))))

(fn `UserConstructionScript`
  (`parent.UserConstructionScript`))
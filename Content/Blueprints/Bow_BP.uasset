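; VR bow that spawns, aims and fires an Arrow_BP through a grabbable child-actor string handle.
; Each Tick, handle travel becomes a pull percentage that drives the string AnimBP.
; While held, the arrow follows the handle along the bow's clamped X axis, offset by hand side, and a line trace draws a debug aim point.
; Release applies a pull-scaled physics impulse along the bow's negative forward vector, plus scaled haptic feedback.
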(event `self.ReceiveBeginPlay`
  (`|ExecutionSequence`
    (:`then_0`
      (bind _asbow_string_anim_bp (cast `/Game/Models/Bow_String_AnimBP` (`SkeletalMeshComponent.GetAnimInstance` (`self.SkeletalMeshComponent`))))
      (set `self.AnimBP` _asbow_string_anim_bp))
    (:`then_1`
      (bind _asstring_handle_bp (cast `/Game/Blueprints/StringHandle_BP` (`ChildActorComponent.ChildActor` (`self.StringHandleActor`))))
      (set `self.StringHanlde` _asstring_handle_bp))))

(event `self.ReceiveTick`
  (params (DeltaSeconds :type "Float (single-precision)"))
  (bind _stringhanlde (`self.StringHanlde`))
  (bind _arrow_bp (`self.Arrow_BP`))
  (bind _grabcomponent (`/Game/Blueprints/StringHandle_BP.GrabComponent` _stringhanlde))
  (bind _returnvalue (`KismetMathLibrary.MakeTransform` (`self.K2_GetActorLocation` (`self.StringHanlde`)) (`self.K2_GetActorRotation`)))
  (`self.Update String Animation` _stringhanlde)
  (if (`/Game/VRTemplate/Blueprints/GrabComponent.bIsHeld` _grabcomponent)
    (`|ExecutionSequence`
      (:`then_0`
        (`/Engine/EditorBlueprintResources/StandardMacros.DoOnce` false :!label _label
          (:`Completed`
            (set `self.StringHold` true)
            (set `self.HeldHand` (`/Game/VRTemplate/Blueprints/GrabComponent.GetHeldByHand` _grabcomponent))
            ;[1 1 1] Create Arrow
            (`KismetSystemLibrary.PrintString` "Arrow Spawn")
            (bind _returnvalue_2 (`|SpawnActorFromClass` "/Game/Blueprints/Arrow_BP.Arrow_BP_C" _returnvalue "AlwaysSpawn" "MultiplyWithRoot" null null))
            (set `self.Arrow_BP` _returnvalue_2))))
      (:`then_1`
        ;[1 1 1] Update Arrow Position
        (`self.UpdateArrowTransform` _returnvalue))
      (:`then_2`
        (`self.Aimming`)))
    (else
      (`|ExecutionSequence`
        (:`then_0`
          (goto _label :!via `Reset`))
        (:`then_1`
          (if (`self.StringHold`)
            (set `self.StringHold` false)
            ;[1 1 1] Shoot Arrow
            (`KismetSystemLibrary.PrintString` "ShootArrow")
            (`/Game/Blueprints/Arrow_BP.PreparePhysics` _arrow_bp)
            (bind _percent (`self.GetStringPercent` _stringhanlde))
            (`self.ShootArrow` (`KismetMathLibrary.Lerp` 0.0 (`self.MaxStringForce`) _percent))
            (`/Game/Blueprints/Arrow_BP.OnShootEN_Event` _arrow_bp)
            (`PlayerController.PlayHapticEffect` (`GameplayStatics.GetPlayerController` 0) "/Game/VR_Haptics/Bow/PistolFireHapticEffect.PistolFireHapticEffect" (`/Game/VRTemplate/Blueprints/GrabComponent.GetHeldByHand` (`/Game/Blueprints/StringHandle_BP.GrabComponent` (`self.StringHanlde`))) (`KismetMathLibrary.Lerp` 0.5 3.0 _percent) false)))))))

(fn `Aimming`
  (locals (rayLength :type "Float (double-precision)" :default 1000.0))
  (bind _arrow_bp (`self.Arrow_BP`))
  (bind _returnvalue (`SceneComponent.K2_GetComponentLocation` (`/Game/Blueprints/Arrow_BP.ArrowTail` _arrow_bp)))
  (bind (_outhit _returnvalue_2) (`KismetSystemLibrary.LineTraceSingle` _returnvalue (+ _returnvalue (* (`self.GetActorForwardVector` _arrow_bp) (* (`local.rayLength`) -1.0))) "TraceTypeQuery1" false (`|MakeArray` _arrow_bp :!type "Actor Object Reference")))
  (if _returnvalue_2
    (`KismetSystemLibrary.DrawDebugPoint` (`.Location` (`GameplayStatics.BreakHitResult` _outhit)) 10.0 (struct :`R` 1.0 :`A` 1.0))))

(fn `GetStringPercent`
  (params (StringHandle :type "/Game/Blueprints/StringHandle_BP Object Reference"))
  (returns (percent :type "Float (double-precision)"))
  (bind _lengthalongaxis (`/Game/Blueprints/StringHandle_BP.Get Length Along Axis` StringHandle))
  (return (`KismetMathLibrary.FClamp` (/ _lengthalongaxis 50.0))))

(fn `ShootArrow`
  (params (Force :type "Float (double-precision)"))
  (bind _arrow_bp (`self.Arrow_BP`))
  (if (`KismetSystemLibrary.IsValid` _arrow_bp)
    (`PrimitiveComponent.AddImpulse` (`/Game/Blueprints/Arrow_BP.StaticMesh` _arrow_bp) (* (`self.GetActorForwardVector`) (* Force -1.0)) "None" false)))

(fn `Update String Animation`
  (params (StringHandle :type "/Game/Blueprints/StringHandle_BP Object Reference"))
  ;[1 1 1] String Animation
  (bind _percent (`self.GetStringPercent` StringHandle))
  (bind _output_get (set `self.percent` _percent))
  (set `/Game/Models/Bow_String_AnimBP.SliderProgress` _output_get (`self.AnimBP`)))

(fn `UpdateArrowTransform`
  (params (HandleTransform :type "Transform Structure"))
  (locals (Offset :type "Float (double-precision)" :default 3.0) (sign :type "Float (double-precision)"))
  (bind _returnvalue (`self.GetTransform`))
  (bind _rotation (.rotation HandleTransform))
  (bind _scale (.scale HandleTransform))
  (bind _returnvalue_2 (`KismetMathLibrary.TransformLocation` _returnvalue (`KismetMathLibrary.MakeVector` (`KismetMathLibrary.FClamp` (.x (`KismetMathLibrary.InverseTransformLocation` _returnvalue (.location HandleTransform))) (`self.ArrowOffsetMin`) (`self.ArrowOffsetMax`)) 0.0 (* (`local.sign`) (`local.Offset`)))))
  (switch `EControllerHand` (`self.HeldHand`)
    (:`Left`
      (set `local.sign` -1.0)
      (`self.K2_SetActorTransform` (`self.Arrow_BP`) (`KismetMathLibrary.MakeTransform` _returnvalue_2 _rotation _scale) false true))
    (:`Right`
      (set `local.sign` 1.0)
      (`self.K2_SetActorTransform` (`self.Arrow_BP`) (`KismetMathLibrary.MakeTransform` _returnvalue_2 _rotation _scale) false true))))

(fn `UserConstructionScript`)
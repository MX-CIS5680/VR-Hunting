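; Physics-driven arrow that can pierce Target_BP actors or be blocked by them, and destroys itself five seconds after being shot.
; On overlap, a line trace from the tail finds the surface normal, and normal-direction speed is tested against the target's threshold.
; A piercing arrow notifies and attaches to the target, then Tick applies the target's damping until it stops; otherwise collision switches to blocking.
; Movable simulating components receive a momentum-based impulse.
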(event `self.ReceiveBeginPlay`
  (add `self.OnShootEN` (delegate `OnShootEN_Event`)))

(event `OnShootEN_Event`
  (`|ExecutionSequence`
    (:`then_1`
      (`KismetSystemLibrary.Delay` 5.0)
      (`SceneComponent.K2_DetachFromComponent` (`self.StaticMesh`) "KeepRelative" "KeepRelative" "KeepRelative" true)
      (`self.K2_DestroyActor`))))

(event `self.ReceiveTick`
  (params (DeltaSeconds :type "Float (single-precision)"))
  (if (`self.IsBreakThrough`)
    (`self.ReduceVelocity` (`/Game/Blueprints/Target_BP.Damping` (`self.TargetBP`)) DeltaSeconds)
    (`self.CheckStop`)))

(event `self.StaticMesh.OnComponentBeginOverlap`
  (params (OverlappedComponent :type "PrimitiveComponent Object Reference") (OtherActor :type "Actor Object Reference") (OtherComp :type "PrimitiveComponent Object Reference") (OtherBodyIndex :type Integer) (bFromSweep :type Boolean) (SweepResult :type "HitResult Structure (by ref)"))
  (if (`self.TestOverlap`)
    (bind _astarget_bp (cast `/Game/Blueprints/Target_BP` OtherActor))
    (bind _hitresult (`self.GetHitResult`))
    (bind (_bblockinghit _binitialoverlap _time _distance _location _impactpoint _normal) (`GameplayStatics.BreakHitResult` _hitresult))
    (bind _breakthrough (`self.BreakThrough` _normal (`/Game/Blueprints/Target_BP.Threshold` _astarget_bp)))
    (set `self.TestOverlap` false)
    (`self.AddImpulse` _location OtherComp)
    (if _breakthrough
      (bind _returnvalue (`PrimitiveComponent.GetPhysicsLinearVelocity` (`self.StaticMesh`) "None"))
      (`/Game/Blueprints/Target_BP.OnShooted` _astarget_bp _location _normal _returnvalue)
      (`PrimitiveComponent.SetEnableGravity` (`self.StaticMesh`) false)
      (set `self.TargetBP` _astarget_bp)
      (set `self.IsBreakThrough` true)
      (`self.AttachToTarget`)
      (else
        (`self.Blocked`)))))

(event `self.StaticMesh.OnComponentHit`
  (params (HitComponent :type "PrimitiveComponent Object Reference") (OtherActor :type "Actor Object Reference") (OtherComp :type "PrimitiveComponent Object Reference") (NormalImpulse :type "Vector Structure") (Hit :type "HitResult Structure (by ref)"))
  (set `self.TestOverlap` false))

(fn `AddImpulse`
  (params (Location :type "Vector Structure") (component :type "PrimitiveComponent Object Reference"))
  (bind _staticmesh (`self.StaticMesh`))
  (if (`SceneComponent.IsSimulatingPhysics` component "None")
    (switch `EComponentMobility` (`SceneComponent.Mobility` component)
      (:`Movable`
        (bind _returnvalue (`PrimitiveComponent.GetPhysicsLinearVelocity` _staticmesh "None"))
        (`PrimitiveComponent.AddImpulseAtLocation` component (* _returnvalue (`PrimitiveComponent.GetMass` _staticmesh)) Location "None")))))

(fn `AttachToTarget`
  (locals (tempTrans :type "Transform Structure"))
  (bind _staticmesh (`self.StaticMesh`))
  (set `local.tempTrans` (`SceneComponent.K2_GetComponentToWorld` _staticmesh))
  (`SceneComponent.K2_AttachToComponent` _staticmesh (`/Game/Blueprints/Target_BP.StaticMesh` (`self.TargetBP`)) "None" "KeepRelative" "KeepRelative" "KeepRelative" true)
  (`SceneComponent.K2_SetWorldTransform` _staticmesh (`local.tempTrans`) false true))

(fn `Blocked`
  (`PrimitiveComponent.SetCollisionResponseToChannel` (`self.StaticMesh`) "ECC_GameTraceChannel3" "ECR_Block")
  (`KismetSystemLibrary.PrintString` "Blocked"))

(fn `BreakThrough`
  (params (Normal :type "Vector Structure") (Threshold :type "Float (double-precision)"))
  (returns (breakThrough :type Boolean))
  (bind _returnvalue (`PrimitiveComponent.GetPhysicsLinearVelocity` (`self.StaticMesh`) "None"))
  (bind _returnvalue_2 (`KismetMathLibrary.Abs` (`KismetMathLibrary.Dot_VectorVector` Normal _returnvalue)))
  (`KismetSystemLibrary.PrintString` (`KismetStringLibrary.Conv_DoubleToString` _returnvalue_2) true true (struct :`R` 0.134018 :`G` 1.0 :`B` 0.024775 :`A` 1.0))
  (return (> _returnvalue_2 Threshold)))

(fn `CheckStop`
  (locals (TempTrans :type "Transform Structure"))
  (bind _staticmesh (`self.StaticMesh`))
  (bind _returnvalue (`PrimitiveComponent.GetPhysicsLinearVelocity` _staticmesh "None"))
  (bind _returnvalue_2 (* (`KismetMathLibrary.Dot_VectorVector` (`self.GetActorForwardVector`) _returnvalue) -1.0))
  (`KismetSystemLibrary.PrintString` (`KismetStringLibrary.Conv_DoubleToString` _returnvalue_2))
  (if (<= _returnvalue_2 0.1)
    (`PrimitiveComponent.SetPhysicsLinearVelocity` _staticmesh (0.0 0.0 0.0) false "None")
    (set `self.IsBreakThrough` false)
    (`PrimitiveComponent.SetSimulatePhysics` _staticmesh false)))

(fn `GetHitResult`
  (returns (HitResult :type "HitResult Structure"))
  (locals (distance :type "Float (double-precision)" :default 1000.0))
  (bind _arrowtail (`self.ArrowTail`))
  (bind _returnvalue (`SceneComponent.K2_GetComponentLocation` _arrowtail))
  (bind (_outhit _returnvalue_2) (`KismetSystemLibrary.LineTraceSingle` _returnvalue (+ (* (`self.GetActorForwardVector`) (* (`local.distance`) -1.0)) _returnvalue) "TraceTypeQuery1" false (`|MakeArray` (`ActorComponent.GetOwner` _arrowtail))))
  (if (not _returnvalue_2)
    (`KismetSystemLibrary.PrintString` "cast ray failed" true true (struct :`R` 1.0 :`B` 0.030547 :`A` 1.0)))
  (return _outhit))

(fn `OnShoot`)

(fn `PreparePhysics`
  (`PrimitiveComponent.SetSimulatePhysics` (`self.StaticMesh`) true))

(fn `ReduceVelocity`
  (params (Damping :type "Float (double-precision)") (DeltaSecond :type "Float (double-precision)"))
  (bind _staticmesh (`self.StaticMesh`))
  (bind _returnvalue (`PrimitiveComponent.GetPhysicsLinearVelocity` _staticmesh "None"))
  (`PrimitiveComponent.SetPhysicsLinearVelocity` _staticmesh (* (`KismetMathLibrary.Normal` _returnvalue) (* (* Damping DeltaSecond) -1.0)) true "None"))

(fn `UserConstructionScript`)
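; StringHandle is a grabbable string handle child actor that springs back to its rest position on its parent when released.
; BeginPlay caches its parent-relative transform, and while held Tick locks its rotation to that rest pose.
; On release, a DoOnce-gated short timeline eases it home with grabbing disabled, then Tick pins it to the parent.
; GetLengthAlongAxis measures pull distance from rest along a selectable local axis.
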(event `self.ReceiveBeginPlay`
  (set `self.AttachedParent` (`self.GetParentActor`))
  (bind _currentlocaltransform (`self.GetCurrentLocalTransform`))
  (bind _output_get (set `self.InitLocalTrans` _currentlocaltransform))
  (bind _rotation (.rotation _output_get))
  (set `self.InitLocalLocation` (.location _output_get))
  (set `self.InitLocalRotator` _rotation)
  (`KismetSystemLibrary.PrintString` (`KismetStringLibrary.Conv_RotatorToString` _rotation)))

(event `self.ReceiveTick`
  (params (DeltaSeconds :type "Float (single-precision)"))
  (bind _resettoinit (`self.ResetToInit`))
  (if (`/Game/VRTemplate/Blueprints/GrabComponent.bIsHeld` (`self.GrabComponent`))
    (`|ExecutionSequence`
      (:`then_0`
        (goto _label :!via `Reset`))
      (:`then_1`
        ;[1 1 1] Return to original place
        (`self.KeepRelativeRotation`)
        (set `self.Returned` false)))
    (else
      (`|ExecutionSequence`
        (:`then_0`
          (`/Engine/EditorBlueprintResources/StandardMacros.DoOnce` true :!label _label
            (:`Completed`
              (set `/Game/VRTemplate/Blueprints/GrabComponent.IsGrablable` false (`self.GrabComponent`))
              (`|ExecutionSequence`
                (:`then_0`
                  (`TimelineComponent.SetTimelineLength` _resettoinit 0.1)
                  (`Timeline|ResetToInit` :!via `PlayFromStart`
                    (:`Update`
                      (`self.StringReturn` (`TimelineComponent.GetPlaybackPosition` _resettoinit)))
                    (:`Finished`
                      (set `self.Returned` true)
                      (set `/Game/VRTemplate/Blueprints/GrabComponent.IsGrablable` true (`self.GrabComponent`))
                      (`KismetSystemLibrary.PrintString` "Return"))))))))
        (:`then_1`
          (if (`self.Returned`)
            (`self.KeepRelativeTransform`)))))))

(fn `Get Diff in World`
  (returns (WorldDifference :type "Vector Structure"))
  (return (- (`self.K2_GetActorLocation`) (`KismetMathLibrary.TransformLocation` (`self.GetTransform` (`self.AttachedParent`)) (`self.InitLocalLocation`)))))

(fn `Get Length Along Axis`
  (returns (lengthAlongAxis :type "Float (double-precision)"))
  (locals (Length :type "Float (double-precision)"))
  (bind _worlddifference (`self.Get Diff in World`))
  (switch `/Game/Blueprints/Enum/MyAxis` (`self.Axis`)
    (:`NewEnumerator0`
      (bind _output_get (set `local.Length` (`KismetMathLibrary.Dot_VectorVector` _worlddifference (`self.GetActorForwardVector`)))))
    (:`NewEnumerator1`
      (set `local.Length` (`KismetMathLibrary.Dot_VectorVector` _worlddifference (`self.GetActorRightVector`))))
    (:`NewEnumerator2`
      (set `local.Length` (`KismetMathLibrary.Dot_VectorVector` _worlddifference (`self.GetActorUpVector`)))))
  (return (`local.Length`)))

(fn `GetCurrentLocalLocation`
  (returns (CurrentLocalLocation :type "Vector Structure"))
  (return (`KismetMathLibrary.InverseTransformLocation` (`self.GetTransform` (`self.AttachedParent`)) (`self.K2_GetActorLocation`))))

(fn `GetCurrentLocalRotation`
  (returns (CurrentLocalRotation :type "Rotator Structure"))
  (return (`KismetMathLibrary.InverseTransformRotation` (`self.GetTransform` (`self.AttachedParent`)) (`self.K2_GetActorRotation`))))

(fn `GetCurrentLocalTransform`
  (returns (CurrentLocalTransform :type "Transform Structure"))
  (return (`KismetMathLibrary.MakeRelativeTransform` (`self.GetTransform`) (`self.GetTransform` (`self.AttachedParent`)))))

(fn `KeepRelativeRotation`
  (`self.K2_SetActorRotation` (`KismetMathLibrary.TransformRotation` (`self.GetTransform` (`self.AttachedParent`)) (.rotation (`self.InitLocalTrans`))))
  (`/Engine/EditorBlueprintResources/StandardMacros.DoOnce` false))

(fn `KeepRelativeTransform`
  (`self.K2_SetActorTransform` (`KismetMathLibrary.MakeRelativeTransform` (`self.InitLocalTrans`) (`KismetMathLibrary.InvertTransform` (`self.GetTransform` (`self.AttachedParent`)))) false true))

(fn `StringReturn`
  (params (Percent :type "Float (double-precision)"))
  (bind _currentlocallocation (`self.GetCurrentLocalLocation`))
  (`self.K2_SetActorLocation` (+ (`self.K2_GetActorLocation`) (* (`KismetMathLibrary.TransformDirection` (`self.GetTransform` (`self.AttachedParent`)) (- (`self.InitLocalLocation`) _currentlocallocation)) Percent)) false true))

(fn `UserConstructionScript`)
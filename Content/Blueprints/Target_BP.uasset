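; Shooting target that leaves a mark where it is hit and prints how far the hit landed from its Plane component.
; OnShooted spawns an Img actor scaled by CrossScale, nudged along the hit normal by Epsilion and using the target's rotation.
; It attaches the mark to the target, then restores the saved world transform so it stays in place.
; The event graph and construction script are empty.
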(fn `OnShooted`
  (params (HitLocation :type "Vector Structure") (Normal :type "Vector Structure") (Velocity :type "Vector Structure"))
  (locals (crossScale :type "Float (double-precision)" :default 0.1) (epsilion :type "Float (double-precision)" :default 1.0) (tempTrans :type "Transform Structure"))
  (bind _crossscale (`local.crossScale`))
  (`|ExecutionSequence`
    (:`then_0`
      (bind _returnvalue (`|SpawnActorFromClass` "/Game/Blueprints/img.img_C" (`KismetMathLibrary.MakeTransform` (+ HitLocation (* Normal (`local.epsilion`))) (.rotation (`self.GetTransform`)) (`KismetMathLibrary.MakeVector` _crossscale _crossscale _crossscale)) "AlwaysSpawn" "MultiplyWithRoot" null null))
      (set `local.tempTrans` (`self.GetTransform` _returnvalue))
      (`self.K2_AttachToActor` _returnvalue (`ActorComponent.GetOwner` (`self.StaticMesh`)) "None" "KeepRelative" "KeepRelative" "KeepRelative" true)
      (`self.K2_SetActorTransform` _returnvalue (`local.tempTrans`) false true))
    (:`then_1`
      (`KismetSystemLibrary.PrintString` (`KismetStringLibrary.Conv_DoubleToString` (`KismetMathLibrary.VSize` (- HitLocation (`SceneComponent.K2_GetComponentLocation` (`self.Plane`))))) true true (struct :`R` 1.0 :`G` 0.090284 :`A` 1.0)))))

(fn `UserConstructionScript`)